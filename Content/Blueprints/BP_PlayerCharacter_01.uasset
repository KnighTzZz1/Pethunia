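; Player character Blueprint with a hitscan shot and a short "Flash" dash, both aimed along the camera.
; Fire runs a debug-drawn line trace that damages the first PlayerHealthComponent on actors tagged "damagable".
; Flash spends EnergyComponent energy, launches the character at high speed, stops it almost immediately, then waits out a cooldown.
; BeginPlay adds the HUD and hides the mesh when locally controlled.
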(event `InputAction|Fire`
  (params (Key :type "Key Structure"))
  (bind _camera (`self.Camera`))
  (bind _returnvalue (`SceneComponent.K2_GetComponentLocation` _camera))
  (:`Pressed`
    (bind (_outhit _returnvalue_2) (`KismetSystemLibrary.LineTraceSingle` :`Start` _returnvalue :`End` (+ _returnvalue (* (`SceneComponent.GetForwardVector` _camera) 10000.0)) :`TraceChannel` "TraceTypeQuery2" :`DrawDebugType` "ForDuration" :`TraceColor` (struct :`R` 1.0 :`G` 0.20158 :`A` 1.0)))
    (bind (_bblockinghit _binitialoverlap _time _distance _location _impactpoint _normal _impactnormal _physmat _hitactor) (`GameplayStatics.BreakHitResult` _outhit))
    (if (== _hitactor null)
      _
      (elif _returnvalue_2
        (if (`self.ActorHasTag` _hitactor "damagable")
          (`PlayerHealthComponent.TakeDamage` (`|GetArrayItem` (`self.K2_GetComponentsByClass` _hitactor "/Script/Pethunia.PlayerHealthComponent")) 50.0)
          (`KismetSystemLibrary.PrintString` "Actor has taken damage"))))))

(event `Key|F`
  (params (Key :type "Key Structure"))
  (bind _energycomponent (`self.EnergyComponent`))
  (:`Pressed`
    (if (and (>= (`PlayerEnergyComponent.Energy` _energycomponent) 20.0) (not (`self.Flash is on cooldown`)))
      (`PlayerEnergyComponent.UseEnergy` _energycomponent 20.0)
      (set `self.Flash is on cooldown` true)
      (`self.LaunchCharacter` (* (`SceneComponent.GetForwardVector` (`self.Camera`)) 25000.0) true true)
      (`KismetSystemLibrary.Delay` 0.05)
      (`MovementComponent.StopMovementImmediately` (`self.CharacterMovement`))
      (`KismetSystemLibrary.Delay` 1.0)
      (set `self.Flash is on cooldown` false))))

(event `self.ReceiveBeginPlay`
  (bind _returnvalue (`|CreateWidget` "/Game/Widgets/Hud.Hud_C"))
  (`UserWidget.AddToViewport` _returnvalue 0)
  (if (`self.IsLocallyControlled`)
    (`SceneComponent.SetVisibility` (`self.Mesh`) false false)))

(fn `UserConstructionScript`)