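; First-person player character Blueprint, marked old, that handles hitscan firing and local setup.
; Fire line-traces from the camera on the Camera channel, damaging "damagable" actors through their PlayerHealthComponent or spawning falling-leaf particles on "Tree"-tagged components.
; BeginPlay adds the HUD widget without a local-control check, then hides the character mesh only for the locally controlled player.
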(event `InputAction|Fire`
  (params (Key :type "Key Structure"))
  (bind _camera (`self.Camera`))
  (bind _returnvalue (`SceneComponent.K2_GetComponentLocation` _camera))
  (:`Pressed`
    (bind (_outhit _returnvalue_2) (`KismetSystemLibrary.LineTraceSingle` :`Start` _returnvalue :`End` (+ _returnvalue (* (`SceneComponent.GetForwardVector` _camera) 10000.0)) :`TraceChannel` "TraceTypeQuery2" :`TraceColor` (struct :`R` 1.0 :`G` 0.20158 :`A` 1.0)))
    (bind (_bblockinghit _binitialoverlap _time _distance _location _impactpoint _normal _impactnormal _physmat _hitactor _hitcomponent) (`GameplayStatics.BreakHitResult` _outhit))
    (if (== _hitactor null)
      _
      (elif _returnvalue_2
        (if (`self.ActorHasTag` _hitactor "damagable")
          (`PlayerHealthComponent.TakeDamage` (`|GetArrayItem` (`self.K2_GetComponentsByClass` _hitactor "/Script/Pethunia.PlayerHealthComponent")) 50.0)
          (`KismetSystemLibrary.PrintString` "Actor has taken damage")
          (elif (`ActorComponent.ComponentHasTag` _hitcomponent "Tree")
            (`GameplayStatics.SpawnEmitterAtLocation` "/Game/Particles/PS_FallingLeaves.PS_FallingLeaves" _location)))))))

(event `self.ReceiveBeginPlay`
  (bind _returnvalue (`|CreateWidget` "/Game/Widgets/Hud.Hud_C"))
  (`UserWidget.AddToViewport` _returnvalue 0)
  (if (`self.IsLocallyControlled`)
    (`SceneComponent.SetVisibility` (`self.Mesh`) false false)))

(fn `UserConstructionScript`)