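; BP_HighMobilityPlayer is a player pawn Blueprint with health and energy components and a HUD.
; On BeginPlay it creates the HUD widget, adds it to the viewport, and hides the body mesh for the locally controlled player.
; The E and F keys directly apply fixed damage to HealthComponent and spend a fixed amount from EnergyComponent.
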(event `Key|E`
  (params (Key :type "Key Structure"))
  (:`Pressed`
    (`PlayerHealthComponent.TakeDamage` (`self.HealthComponent`) 10.0)))

(event `Key|F`
  (params (Key :type "Key Structure"))
  (:`Pressed`
    (`PlayerEnergyComponent.UseEnergy` (`self.EnergyComponent`) 15.0)))

(event `self.ReceiveBeginPlay`
  (bind _returnvalue (`|CreateWidget` "/Game/Widgets/Hud.Hud_C"))
  (`UserWidget.AddToViewport` _returnvalue 0)
  (if (`self.IsLocallyControlled`)
    (`SceneComponent.SetVisibility` (`self.Mesh`) false false)))

(fn `UserConstructionScript`)