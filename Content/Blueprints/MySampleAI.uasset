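; MySampleAI is a Blueprint that pushes its static mesh along a looping force pattern sampled from a curve.
; On BeginPlay a repeating timer calls IncreaseTime, which advances a Time value and wraps it to zero at the curve's end.
; Each step applies the scaled vector from Curvex as a physics force on the mesh.
; BeginPlay also stores a next butterfly destination, which nothing here reads.
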(event `self.ReceiveBeginPlay`
  (set `self.NextButterflyDestination` (0.0 3647.0 -3273.0))
  (`KismetSystemLibrary.K2_SetTimer` null "IncreaseTime" 0.1 true))

(fn `IncreaseTime`
  (bind _curvex (`self.Curvex`))
  (if (>= (`self.Time`) (`.MaxTime` (`CurveBase.GetTimeRange` _curvex)))
    (set `self.Time` 0.0)
    (else
      (bind _output_get (set `self.Time` (+ (`self.Time`) (`self.Time Offset`))))
      (`PrimitiveComponent.AddForce` (`self.StaticMesh`) (* (`CurveVector.GetVectorValue` _curvex _output_get) 150.0) "None" false))))

(fn `UserConstructionScript`)