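; Deathmatch game mode that starts the match with two or more players or after a fixed BeginPlay delay.
; PostLogin stores each controller and uses its list index as player ID, setting it and a random colour on BP_PlayerState.
; Deaths trigger a delayed respawn at a random spot from externally registered start positions.
; Tick polls BP_GameState and restarts the game when round time hits zero.
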(event `Assign Player Colour And Index`
  (params (Controller :type "PlayerController Object Reference") (ID :type Integer))
  (bind (_returnvalue_x _returnvalue_y _returnvalue_z) (`KismetMathLibrary.BreakVector` (`KismetMathLibrary.RandomUnitVector`)))
  (bind _asbp_player_state (cast `/Game/Blueprints/BP_PlayerState` (`Controller.PlayerState` Controller))
    (:`then`
      (`/Game/Blueprints/BP_PlayerState.Set Player Color` _asbp_player_state (`KismetMathLibrary.Conv_LinearColorToColor` (`KismetMathLibrary.MakeColor` _returnvalue_x _returnvalue_y _returnvalue_z)))
      (`/Game/Blueprints/BP_PlayerState.Set Player ID` _asbp_player_state ID))
    (:`CastFailed`
      (`KismetSystemLibrary.PrintString` "Cast To BP_PlayerState Failed"))))

(event `self.K2_PostLogin`
  (params (NewPlayer :type "PlayerController Object Reference"))
  (bind _returnvalue (`KismetArrayLibrary.Array_Add` (`self.ControllerList`) NewPlayer))
  (`self.Assign Player Colour And Index` NewPlayer _returnvalue))

(event `self.ReceiveBeginPlay`
  (`KismetSystemLibrary.PrintString` (`KismetStringLibrary.Concat_StrStr` "Has Match Started: " (`KismetStringLibrary.Conv_BoolToString` (`self.HasMatchStarted`))))
  (`KismetSystemLibrary.Delay` 25.0)
  (`self.StartMatch`)
  (`KismetSystemLibrary.PrintString` (`KismetStringLibrary.Concat_StrStr` "Has Match Started: " (`KismetStringLibrary.Conv_BoolToString` (`self.HasMatchStarted`)))))

(event `Add Start Position Server`
  (params (`Start Position` :type "PlayerStart Object Reference"))
  (`KismetArrayLibrary.Array_Add` (`self.Start Positions`) `Start Position`))

(event `self.ReceiveTick`
  (params (DeltaSeconds :type "Float (single-precision)"))
  (bind _asbp_game_state (cast `/Game/Blueprints/BP_GameState` (`GameplayStatics.GetGameState`)))
  (bind _round_time (`/Game/Blueprints/BP_GameState.Get Round Time` _asbp_game_state))
  (if (== _round_time 0)
    (`self.RestartGame`)))

(event `OnPlayerDeath`
  (params (`Player ID` :type Integer))
  (bind _start_positions (`self.Start Positions`))
  (`KismetSystemLibrary.Delay` (`self.Respawn Delay`))
  (`self.RestartPlayerAtPlayerStart` (`|GetArrayItem` (`self.ControllerList`) `Player ID`) (`|GetArrayItem` _start_positions (`KismetMathLibrary.RandomInteger` (`KismetArrayLibrary.Array_Length` _start_positions)))))

(fn `ReadyToStartMatch`
  (returns (ReturnValue :type Boolean))
  (return (>= (`KismetArrayLibrary.Array_Length` (`self.ControllerList`)) 2)))

(fn `UserConstructionScript`)