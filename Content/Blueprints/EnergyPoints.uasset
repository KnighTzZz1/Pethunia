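; Energy pickup actor that grants energy to the player when touched, then destroys itself.
; Tick spins it on roll and yaw and plays a timeline whose track incrementally offsets its height.
; An overlap by a Player-tagged actor calls GetEnergy on player 0's EnergyComponent with a fixed amount and spawns a pickup particle effect.
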(event `self.ReceiveTick`
  (params (DeltaSeconds :type "Float (single-precision)"))
  (`self.K2_SetActorRotation` (`KismetMathLibrary.MakeRotator` (+ (.roll (`self.K2_GetActorRotation`)) 0.5) 0.0 (+ (.yaw (`self.K2_GetActorRotation`)) 0.5)))
  (bind (_direction _newtrack_0) (`Timeline|Timeline_0`)
    (:`Update`
      (`self.K2_SetActorLocation` (`KismetMathLibrary.MakeVector` (.x (`self.K2_GetActorLocation`)) (.y (`self.K2_GetActorLocation`)) (+ (.z (`self.K2_GetActorLocation`)) (/ _newtrack_0 2.0)))))))

(event `self.ReceiveActorBeginOverlap`
  (params (OtherActor :type "Actor Object Reference"))
  (if (`self.ActorHasTag` OtherActor "Player")
    (bind _asbp_player_character_01 (cast `/Game/Blueprints/BP_PlayerCharacter_01` (`GameplayStatics.GetPlayerCharacter` 0)))
    (bind _energycomponent (`PlayerCharacter.EnergyComponent` _asbp_player_character_01))
    (if (not (== _energycomponent null))
      (`PlayerEnergyComponent.GetEnergy` _energycomponent 25.0)
      (`GameplayStatics.SpawnEmitterAtLocation` "/Game/Particles/PS_EnergyPickup.PS_EnergyPickup" (`self.K2_GetActorLocation`))
      (`self.K2_DestroyActor`))))

(fn `UserConstructionScript`)