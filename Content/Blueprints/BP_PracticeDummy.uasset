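; BP_PracticeDummy is a practice dummy actor with two custom events that recolor its DummyMesh.
; Each event creates a dynamic material instance from TestMaterial, sets its BodyColor parameter and applies it to the mesh.
; ChangeColorMulticast turns the body green and ChangeColorServer turns it red, with names suggesting a replication test.
; BeginPlay reaches an authority switch with nothing connected after it, and nothing here calls either color event.
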(event `Change Color Multicast`
  (bind _returnvalue (`KismetMaterialLibrary.CreateDynamicMaterialInstance` "/Game/Materials/BasicMaterials/TestMaterial.TestMaterial"))
  (`MaterialInstanceDynamic.SetVectorParameterValue` _returnvalue "BodyColor" (struct :`G` 0.84375 :`B` 0.059511 :`A` 1.0))
  (`PrimitiveComponent.SetMaterial` (`self.DummyMesh`) 0 _returnvalue))

(event `Change Color Server`
  (bind _returnvalue (`KismetMaterialLibrary.CreateDynamicMaterialInstance` "/Game/Materials/BasicMaterials/TestMaterial.TestMaterial"))
  (`MaterialInstanceDynamic.SetVectorParameterValue` _returnvalue "BodyColor" (struct :`R` 0.84375 :`B` 0.09547 :`A` 1.0))
  (`PrimitiveComponent.SetMaterial` (`self.DummyMesh`) 0 _returnvalue))

(event `self.ReceiveBeginPlay`
  (`/Engine/EditorBlueprintResources/ActorMacros.Switch Has Authority`))

(fn `UserConstructionScript`)