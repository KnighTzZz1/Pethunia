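; BP_PrimaryGameMode is a game mode Blueprint that records the player count and handles delayed player respawns.
; On BeginPlay it sets RoundTime, waits briefly, then stores the current player count in MaxNumPlayers and prints it.
; The custom event "bla" prints a revive message, restarts the given player after a five-second delay, then increments MaxNumPlayers.
; RoundTime is not used elsewhere in these graphs.
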(event `self.ReceiveBeginPlay`
  (set `self.Round Time` 30.0)
  (`KismetSystemLibrary.Delay` 1.0)
  (bind _returnvalue (`self.GetNumPlayers`))
  (bind _output_get (set `self.Max Num Players` _returnvalue))
  (`KismetSystemLibrary.PrintString` (`KismetStringLibrary.Conv_IntToString` _output_get)))

(event `bla`
  (params (Player :type "Controller Object Reference"))
  (`KismetSystemLibrary.PrintString` "Reviving in 5 seconds")
  (`KismetSystemLibrary.Delay` 5.0)
  (`self.RestartPlayer` Player)
  (`/Engine/EditorBlueprintResources/StandardMacros.IncrementInt` (`self.Max Num Players`)))

(fn `UserConstructionScript`)